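; Passive health regeneration ability that restores health to the affected object in fixed increments over a limited run.
; On apply, it reads AbilityCooldown from the HealthRegeneration data table row as a tick limit and starts a looping half-second timer.
; Each PassiveAbility call sends a health message and increments a counter.
; At the limit, it clears the timer, resets the counter and notifies the owning player's ability handler that it ended.
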(fn ApplyAbility
  (|CallParentFunction)
  (bind _returnvalue (Utilities|GetDataTableRow (Variables|Default|GetAbilityDataTable) "HealthRegeneration")
    (:then
      (Variables|Default|SetMaxCount (Utilities|Struct|BreakS_PassiveAbility _returnvalue))
      (bind _returnvalue_2 (Utilities|Time|SetTimerbyEvent (EventDispatchers|CreateEvent :!event PassiveAbility) 0.5 true))
      (Variables|Default|SetCallPassiveTimer _returnvalue_2))))

(fn PassiveAbility
  (|CallParentFunction)
  (Class|BPIHealthComponent|RecieveHealth(Message) (Variables|Default|GetAffectedObject) "NewEnumerator0" 5.0)
  (Math|Integer|IncrementInt (Variables|Default|GetHealthCount)
    (:%20%20
      (if (== (Variables|Default|GetHealthCount) (Variables|Default|GetMaxCount))
        (Utilities|Time|ClearandInvalidateTimerbyHandle (Variables|Default|GetCallPassiveTimer))
        (Variables|Default|SetHealthCount 0)
        (Default|CallAbilityEnd (CallFunction|GetPlayerAbility (Variables|Default|GetOwningPlayer)) (Variables|Default|GetAbilityType))))))