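; Passive ability that boosts the damage of the owning player's weapon by a multiplier.
; On apply, it binds an event to the inventory's weapon-added dispatcher and runs the passive effect on the active weapon, if valid.
; The boost calls the weapon's IsAffected with its damage plus that damage scaled by DamageMultiplier, so the multiplier acts as a fractional bonus.
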(fn PassiveAbility
  (|CallParentFunction)
  (bind _activeweapon (Class|BPICharacter|GetActiveWeapon(Message) (Variables|Default|GetOwningPlayer)))
  (Utilities|IsValid _activeweapon
    (:Is%20Valid
      (CallFunction|MultiplierDamage _activeweapon))))

(fn ApplyAbility
  (|CallParentFunction)
  (EventDispatchers|BindEventtoWeaponAdded (CallFunction|GetPlayerInventory (Variables|Default|GetOwningPlayer)) (EventDispatchers|CreateEvent :!event MultiplierDamage))
  (CallFunction|PassiveAbility))

(fn MultiplierDamage
  (params (AddedWeapon :type BP%20Weapon%20Base%20Object%20Reference))
  (bind _damage (Variables|/Game/Blueprints/Interactable/Weapons/BP_WeaponBase.BP_WeaponBase_C|GetDamage AddedWeapon))
  (Default|CallIsAffected? AddedWeapon true (+ _damage (* _damage (Variables|Default|GetDamageMultiplier)))))