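; BP_MultiplySpeed is a passive ability that temporarily multiplies the owning player's walk speed.
; ApplyAbility reads the MultiplySpeed data table row, uses its AbilityCooldown as the duration, then triggers ApplyPassiveAbility.
; PassiveAbility caches the current MaxWalkSpeed and scales it by Multiplier.
; After the delay, the event restores the cached speed.
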(event Custom|ApplyPassiveAbility
  (CallFunction|PassiveAbility)
  (Utilities|FlowControl|Delay (Variables|Default|GetDuration))
  (Variables|/Script/Engine.CharacterMovementComponent|SetMaxWalkSpeed (Variables|/Script/Engine.Character|GetCharacterMovement (Variables|Default|GetOwningPlayer)) (Variables|Default|GetOldWalkSpeed)))

(fn ApplyAbility
  (|CallParentFunction)
  (bind _returnvalue (Utilities|GetDataTableRow (Variables|Default|GetAbilityDataTable) "MultiplySpeed")
    (:then
      (Variables|Default|SetDuration (Math|Conversions|ToFloat(Integer) (Utilities|Struct|BreakS_PassiveAbility _returnvalue)))
      (CallFunction|ApplyPassiveAbility))))

(fn PassiveAbility
  (bind _owningplayer (Variables|Default|GetOwningPlayer))
  (bind _charactermovement (Variables|/Script/Engine.Character|GetCharacterMovement _owningplayer))
  (|CallParentFunction)
  (Variables|Default|SetOldWalkSpeed (Variables|/Script/Engine.CharacterMovementComponent|GetMaxWalkSpeed _charactermovement))
  (Variables|/Script/Engine.CharacterMovementComponent|SetMaxWalkSpeed _charactermovement (CallFunction|Multiplier (Variables|/Script/Engine.CharacterMovementComponent|GetMaxWalkSpeed _charactermovement) (Variables|Default|GetMultiplier))))