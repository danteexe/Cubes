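; Blueprint function library of ability helpers, mainly for computing dash launch velocity.
; SelectDashLocation picks the target's last movement input vector, falling back to the mesh's forward vector when that input is zero.
; GetLaunchVelocity normalizes that direction, scales it by the given speed and returns only the horizontal X and Y components.
; A separate Multiplier helper increases a value by a given fraction of itself.
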(fn SelectDashLocation
  (params (TargetObject :type Character%20Object%20Reference))
  (bind _returnvalue (Class|Pawn|GetLastMovementInputVector TargetObject))
  (if (Class|KismetMathLibrary|EqualExactlyVectorVector _returnvalue "0, 0, 0")
    (return (Math|Vector|GetForwardVector (Variables|/Script/Engine.Character|GetMesh TargetObject)))
    (else
      (return _returnvalue))))

(fn GetLaunchVelocity
  (params (TargetObject :type Character%20Object%20Reference) (LaunchVelocity :type Float%20%28single-precision%29))
  (bind _returnvalue (CallFunction|SelectDashLocation TargetObject))
  (bind _returnvalue_2 (Math|Vector|Normalize _returnvalue))
  (bind _returnvalue_3 (* _returnvalue_2 LaunchVelocity))
  (return (.x _returnvalue_3) (.y _returnvalue_3)))

(fn Multiplier
  (params (Value :type Float%20%28single-precision%29) (Multiplier :type Float%20%28single-precision%29))
  (return (+ Value (* Value Multiplier))))