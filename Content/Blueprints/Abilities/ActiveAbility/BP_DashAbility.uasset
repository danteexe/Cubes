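; Active dash ability that launches the owning player with a fixed upward boost when activated.
; ApplyAbility loads dash power and cooldown from the ability's data table row, then starts the active ability, which fires the dash event.
; A DoOnce gate followed by a delay enforces the cooldown before the dash can trigger again.
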(event Custom|StartDashAbility
  (bind _skillprop (Variables|Default|GetSkillProp))
  (bind _owningplayer (Variables|Default|GetOwningPlayer))
  (bind _dashpower (Utilities|Struct|BreakS_ActiveAbility _skillprop))
  (bind (_x _y) (CallFunction|GetLaunchVelocity _owningplayer _dashpower))
  (Utilities|FlowControl|DoOnce false :!label _label
    (:Completed
      (Character|LaunchCharacter _owningplayer (Math|Vector|MakeVector _x _y 2e+02) false false)
      (Utilities|FlowControl|Delay (Utilities|Struct|BreakS_ActiveAbility (Variables|Default|GetSkillProp)))
      (goto _label Reset))))

(fn ApplyAbility
  (bind _abilitydata (Variables|Default|GetAbilityData))
  (|CallParentFunction)
  (bind _returnvalue (Utilities|GetDataTableRow (.datatable _abilitydata) (.rowname _abilitydata))
    (:then
      (Variables|Default|SetSkillProp _returnvalue)
      (CallFunction|StartActiveAbility))))

(fn StartActiveAbility
  (|CallParentFunction)
  (CallFunction|StartDashAbility))