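; BP_DamageAround is a special ability that damages pawns around the owning player.
; Applying it immediately starts the ability, which runs a multi sphere trace at the player's location with debug drawing on.
; Each hit actor takes fixed damage.
; The ability end is signalled to the player's ability component inside the hit loop, so it fires per hit and not at all without hits.
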(fn ApplyAbility
  (|CallParentFunction)
  (CallFunction|StartSpecialAbility))

(fn StartSpecialAbility
  (bind _owningplayer (Variables|Default|GetOwningPlayer))
  (bind _returnvalue (Transformation|GetActorLocation _owningplayer))
  (|CallParentFunction)
  (bind _outhits (Collision|MultiSphereTraceForObjects _returnvalue _returnvalue 5e+02 (Utilities|Array|MakeArray "ObjectTypeQuery3") false 0 "ForDuration"))
  (for _array_element _outhits
    (Game|Damage|ApplyDamage (.HitActor (Collision|BreakHitResult _array_element)) 2e+02 0 0)
    (Default|CallAbilityEnd (CallFunction|GetPlayerAbility (Variables|Default|GetOwningPlayer)) (Variables|Default|GetAbilityType))))