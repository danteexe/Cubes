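; Health component that tracks the owning player's current health and signals death.
; On BeginPlay it binds to the player's OnTakeAnyDamage event and feeds incoming damage into RecieveHealth.
; That function adds or subtracts the value by type (regeneration or damage), clamps the result between zero and MaxHealth, and calls the PlayerDie dispatcher when health is zero.
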(event Custom|OnTakeAnyDamage
  (params (DamagedActor :type Actor%20Object%20Reference) (Damage :type Float%20%28single-precision%29) (DamageType :type Damage%20Type%20Object%20Reference) (InstigatedBy :type Controller%20Object%20Reference) (DamageCauser :type Actor%20Object%20Reference))
  (CallFunction|RecieveHealth "NewEnumerator1" Damage))

(event EventBeginPlay
  (|CallParentFunction)
  (EventDispatchers|AssignOnTakeAnyDamage (Variables|Default|GetOwningPlayer) (delegate Custom|OnTakeAnyDamage)))

(event EventTick
  (params (DeltaSeconds :type Float%20%28single-precision%29)))

(fn RecieveHealth
  (params (RecieveType :type E_HealthRecieveType%20Enum :default "E_AddHealthType_MAX") (Value :type Float%20%28single-precision%29))
  (bind _output_get (Variables|Default|SetCurrentHealth (Math|Float|Clamp(Float) (+ (Variables|Default|GetCurrentHealth) (* Value (Utilities|Select :Index RecieveType :NewEnumerator0 1.0 :NewEnumerator1 -1.0))) 0.0 (Variables|Default|GetMaxHealth))))
  (if (== _output_get 0.0)
    (Default|CallPlayerDie)))