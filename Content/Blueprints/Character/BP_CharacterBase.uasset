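; Base player character that creates the HUD on BeginPlay and updates weapon rotation every tick.
; Enhanced Input actions route weapon equip and drop to ACInventory and primary or special abilities to ACAbilities.
; Shooting messages the active weapon and plays a fire montage, while interacting messages the nearest overlapping BP_InteractableBase.
; Also includes a data-table ability lookup and a work-in-progress store menu on the B key.
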(event EventBeginPlay
  ;[0.1875 0.1875 0.1875 1 30] BeginPlay
  (|CallParentFunction)
  (bind _returnvalue (UserInterface|CreateWidget "/Game/Blueprints/Widget/WBP_Hud.WBP_Hud_C"))
  (Variables|Default|SetHudWidget _returnvalue)
  (UserInterface|Viewport|AddtoViewport (Variables|Default|GetHudWidget) 0))

(event Collision|EventActorBeginOverlap
  (params (OtherActor :type Actor%20Object%20Reference))
  (|CallParentFunction OtherActor) ; This node is disabled and will not be called.\nDrag off pins to build functionality.
)

(event EventTick
  (params (DeltaSeconds :type Float%20%28single-precision%29))
  ;[0.2135 0.2135 0.2135 1 30] Tick
  (|CallParentFunction DeltaSeconds)
  (CallFunction|SetWeaponRotation (Variables|Character|GetMesh)))

(event Input|EnhancedActionEvents|EnhancedInputActionIA_DropWeapon
  (params (ActionValue :type Boolean) (ElapsedSeconds :type Float%20%28single-precision%29) (TriggeredSeconds :type Float%20%28single-precision%29))
  ;[0.3281 0 0 1 30] Drop Weapon
  (Default|DropActiveWeapon (Variables|Default|GetAC_Inventory)))

(event Input|EnhancedActionEvents|EnhancedInputActionIA_Interact
  (params (ActionValue :type Boolean) (ElapsedSeconds :type Float%20%28single-precision%29) (TriggeredSeconds :type Float%20%28single-precision%29))
  ;[0.01388 0.4948 0.005697 1 30] Interact Item
  (Class|BPIInteractable|InteractItem(Message) (.ReturnValue (Actor|FindNearestActor (Transformation|GetActorLocation) (Collision|GetOverlappingActors "/Game/_Core/Blueprints/Interactable/BP_InteractableBase.BP_InteractableBase_C" :!class /Script/Engine.Actor))) self))

(event Input|EnhancedActionEvents|EnhancedInputActionIA_Shoot
  (params (ActionValue :type Boolean) (ElapsedSeconds :type Float%20%28single-precision%29) (TriggeredSeconds :type Float%20%28single-precision%29))
  (bind _activeweapon (CallFunction|GetActiveWeapon))
  ;[0 0.2344 0.2325 1 30] FireWeapon
  (Utilities|IsValid _activeweapon
    (:Is%20Valid
      (Class|BPIWeapon|Shoot(Message) _activeweapon)
      (Animation|Montage|PlayMontage (Variables|Character|GetMesh) "/Game/_Core/Models/Character/Animation/FireAnimation_Montage.FireAnimation_Montage"))))

(event Input|EnhancedActionEvents|EnhancedInputActionIA_EquipPrimaryWeapon
  (params (ActionValue :type Boolean) (ElapsedSeconds :type Float%20%28single-precision%29) (TriggeredSeconds :type Float%20%28single-precision%29))
  ;[0 1 0.9763 1 30] Change Weapon
  (Default|ChangeWeapon (Variables|Default|GetAC_Inventory) "NewEnumerator0"))

(event Input|EnhancedActionEvents|EnhancedInputActionIA_EquipSecondaryWeapon
  (params (ActionValue :type Boolean) (ElapsedSeconds :type Float%20%28single-precision%29) (TriggeredSeconds :type Float%20%28single-precision%29))
  ;[0 1 0.9763 1 30] Change Weapon
  (Default|ChangeWeapon (Variables|Default|GetAC_Inventory) "NewEnumerator1"))

(event Input|EnhancedActionEvents|EnhancedInputActionIA_SpecialAbility
  (params (ActionValue :type Boolean) (ElapsedSeconds :type Float%20%28single-precision%29) (TriggeredSeconds :type Float%20%28single-precision%29))
  ;[0 0.2917 0.2917 1 30] Apply GameplayAbility
  (Default|ApplyGameplayAbility (Variables|Default|GetAC_Abilities) "NewEnumerator1"))

(event Input|EnhancedActionEvents|EnhancedInputActionIA_PrimaryAbility
  (params (ActionValue :type Boolean) (ElapsedSeconds :type Float%20%28single-precision%29) (TriggeredSeconds :type Float%20%28single-precision%29))
  ;[0 0.2917 0.2917 1 30] Apply GameplayAbility
  (Default|ApplyGameplayAbility (Variables|Default|GetAC_Abilities) "NewEnumerator0"))

(event Input|KeyboardEvents|B
  (params (Key :type Key%20Structure))
  ;[1 0 0] WIP
  (:Pressed
    (bind _returnvalue (UserInterface|CreateWidget "/Game/Blueprints/Widget/WBP_StoreMenu.WBP_StoreMenu_C"))
    (UserInterface|Viewport|AddtoViewport _returnvalue 0)))

(fn ConstructionScript
  (|CallParentFunction))

(fn GetActiveWeapon
  (return (Variables|/Game/Blueprints/Inventory/AC_Inventory.AC_Inventory_C|GetActiveWeapon (Variables|Default|GetAC_Inventory))))

(fn GetAbility
  (params (StartedAbility :type Data%20Table%20Row%20Handle%20Structure))
  (bind _returnvalue (Utilities|GetDataTableRow (.datatable StartedAbility) (.rowname StartedAbility))
    (:then
      (return _returnvalue))))