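; BP_AIBase is the base character Blueprint for AI, handling what happens when the AI dies.
; When the health component fires its die event, a short downward line trace finds the ground beneath the character.
; A random gift spawner is spawned at that impact point, then the inventory component drops the active weapon.
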(event PlayerDie(HealthComp)
  (bind _returnvalue (Transformation|GetActorLocation))
  (bind (_x _y _z) (Math|Vector|BreakVector _returnvalue))
  (bind _outhit (Collision|LineTraceByChannel _returnvalue (Math|Vector|MakeVector _x _y (- _z 2e+02)) "TraceTypeQuery1" false 0 "None" true "(R=1.000000,G=0.000000,B=0.000000,A=1.000000)" "(R=0.000000,G=1.000000,B=0.000000,A=1.000000)" 1e+01))
  (Game|SpawnActorfromClass "/Game/Blueprints/Interactable/RandomSpawner/BP_RandomGiftSpawner.BP_RandomGiftSpawner_C" (Math|Transform|MakeTransform (.ImpactPoint (Collision|BreakHitResult _outhit)) "0, 0, 0" "1,1,1") "Undefined" 0 0)
  (Default|DropActiveWeapon (Variables|Default|GetAC_Inventory)))

(event EventBeginPlay
  (|CallParentFunction))

(event Collision|EventActorBeginOverlap
  (params (OtherActor :type Actor%20Object%20Reference))
  (|CallParentFunction OtherActor) ; This node is disabled and will not be called.\nDrag off pins to build functionality.
)

(event EventTick
  (params (DeltaSeconds :type Float%20%28single-precision%29))
  (|CallParentFunction DeltaSeconds) ; This node is disabled and will not be called.\nDrag off pins to build functionality.
)

(fn ConstructionScript
  (|CallParentFunction))