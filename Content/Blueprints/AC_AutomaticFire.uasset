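; AC_AutomaticFire is an actor component that gathers nearby enemy targets for its owning character, apparently groundwork for automatic firing.
; BeginPlay caches the BP_CharacterBase owner and its weapon inventory, then starts a looping timer.
; Each tick of that timer sphere-traces around the owner on the Camera channel, adding "Enemy"-tagged actors to Targets without ever removing any.
; No firing logic exists, and rotation toward the first target is disconnected.
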(event Custom|FindTarget
  (bind _returnvalue (Components|GetOwner))
  (bind _returnvalue_2 (Transformation|GetActorLocation _returnvalue))
  (bind _outhits (Collision|MultiSphereTraceByChannel _returnvalue_2 _returnvalue_2 (Variables|Default|GetTargetRange) "TraceTypeQuery2" false 0 "None" true "(R=1.000000,G=0.000000,B=0.000000,A=1.000000)" "(R=0.000000,G=1.000000,B=0.000000,A=1.000000)" 0.2))
  (for _array_element _outhits
    (Utilities|IsValid (.HitActor (Collision|BreakHitResult _array_element))
      (:Is%20Valid
        (if (Actor|ActorHasTag (.HitActor (Collision|BreakHitResult _array_element)) "Enemy")
          (Utilities|Array|AddUnique (Variables|Default|GetTargets) (.HitActor (Collision|BreakHitResult _array_element))))))))

(event EventBeginPlay
  (Utilities|FlowControl|Sequence
    (:then_0
      (bind _asbp_character_base (Utilities|Casting|CastToBP_CharacterBase (Components|GetOwner)))
      (Variables|Default|SetOwnerCharacter _asbp_character_base)
      (Utilities|IsValid (Variables|/Game/Blueprints/Character/BP_CharacterBase.BP_CharacterBase_C|GetAC_WeaponInventory (Variables|Default|GetOwnerCharacter))
        (:Is%20Valid
          (Variables|Default|SetOwnerInventory (Variables|/Game/Blueprints/Character/BP_CharacterBase.BP_CharacterBase_C|GetAC_WeaponInventory (Variables|Default|GetOwnerCharacter))))
        (:Is%20Not%20Valid
          (Development|PrintString "Owner inventory not valid \\\\\\ AC_ automatic fire"))))
    (:then_1
      (bind _returnvalue (Utilities|Time|SetTimerbyEvent (delegate Custom|FindTarget) 0.1 true))
      (Variables|Default|SetSearchTimerTarget _returnvalue))))

(event EventTick
  (params (DeltaSeconds :type Float%20%28single-precision%29)))