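; Base coin pickup actor that the player collects through an interact event.
; On begin play it rolls a random integer coin value within a fixed range.
; On InteractItem it prints the added amount, passes the value to the game instance through SetCoinMessage, then destroys itself.
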(event EventBeginPlay
  (|CallParentFunction)
  (Variables|Default|SetCoinValue (Math|Random|RandomIntegerinRange 2500 10000)))

(event Collision|EventActorBeginOverlap
  (params (OtherActor :type Actor%20Object%20Reference))
  (|CallParentFunction OtherActor) ; This node is disabled and will not be called.\nDrag off pins to build functionality.
)

(event EventTick
  (params (DeltaSeconds :type Float%20%28single-precision%29))
  (|CallParentFunction DeltaSeconds) ; This node is disabled and will not be called.\nDrag off pins to build functionality.
)

(event EventInteractItem
  (params (Interacter :type Character%20Object%20Reference))
  (Development|PrintString (Utilities|String|Append "Eklenen Tutar" ":" (Utilities|String|ToString(Integer) (Variables|Default|GetCoinValue))))
  (Class|BPIGameInstance|SetCoin(Message) (Game|GetGameInstance) (Variables|Default|GetCoinValue))
  (Actor|DestroyActor))

(fn ConstructionScript
  (|CallParentFunction))