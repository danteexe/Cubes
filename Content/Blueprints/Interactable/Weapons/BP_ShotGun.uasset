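; BP_ShotGun is an interactable shotgun weapon that fires a spread of pellets on each Shoot event.
; Shoot loops once per pellet, running a line trace from the bullet location, playing the shotgun sound and calling DamagePlayer every iteration.
; BulletRange creates the spread by adding a random offset on all three axes to each trace's end point.
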(event EventShoot
  (bind (_start _end) (CallFunction|GetBulletLocation))
  (for _index (range 0 7)
    (CallFunction|SpawnLineTrace _start (+ _end (CallFunction|BulletRange 5e+03)))
    (Audio|PlaySound2D "/Game/Sounds/Judge/ShotgunCue.ShotgunCue" 0.3 1.0 0.0 0 0)
    (CallFunction|DamagePlayer)))

(fn ConstructionScript
  (|CallParentFunction))

(fn BulletRange
  (params (BulletRange :type Float%20%28single-precision%29))
  (bind _returnvalue (* BulletRange -1.0))
  (return (Math|Vector|MakeVector (Math|Random|RandomFloatinRange _returnvalue BulletRange) (Math|Random|RandomFloatinRange _returnvalue BulletRange) (Math|Random|RandomFloatinRange _returnvalue BulletRange))))