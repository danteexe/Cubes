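; Base weapon actor that fires hitscan shots and doubles as an interactable pickup, configured from a data table row on construction.
; Firing runs one debug-drawn line trace per pellet from an arrow, applying base damage or an override while affected.
; Semi fires once; Auto and Burst share a looping timer cleared on stop.
; Interacting drops the interacter's same-type weapon, spawns this one into their inventory and destroys the pickup.
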(event Custom|IsAffected?_Event
  (params (IsAffected :type Boolean) (AffectedProp :type Float%20%28single-precision%29))
  (Variables|Default|SetIs%20Affected IsAffected)
  (Variables|Default|SetAffected%20Damage AffectedProp))

(event EventTick
  (params (DeltaSeconds :type Float%20%28single-precision%29)))

(event EventStartFire
  (switch Utilities|FlowControl|Switch|SwitchonE_FireType (Utilities|Struct|BreakS_WeaponMain (Variables|Default|GetWeaponProp))
    (:NewEnumerator0
      (CallFunction|FireFunction))
    (:NewEnumerator1
      (CallFunction|FireFunction :!label _label)
      (bind _returnvalue (Utilities|Time|SetTimerbyEvent (EventDispatchers|CreateEvent :!event FireFunction) (Utilities|Struct|BreakS_WeaponMain (Variables|Default|GetWeaponProp)) true))
      (Variables|Default|SetAutoFireTimer _returnvalue))
    (:NewEnumerator2
      (goto _label))))

(event EventInteractItem
  (params (Interacter :type Character%20Object%20Reference))
  (bind _returnvalue (Actor|GetComponentbyClass Interacter "/Game/_Core/Blueprints/Component/AC_WeaponInventory.AC_WeaponInventory_C"))
  (bind _weaponprop (Variables|Default|GetWeaponProp))
  ;[0 0.2292 0.227 1 50] Interact Weapon
  (Utilities|IsValid _returnvalue
    (:Is%20Valid
      (Default|DropWeapon _returnvalue (.Value (Utilities|Map|Find (Variables|/Game/_Core/Blueprints/Component/AC_WeaponInventory.AC_WeaponInventory_C|GetEquippedWeapons _returnvalue) (Utilities|Struct|BreakS_WeaponMain (Variables|Default|GetWeaponProp)))))
      (bind _weaponinstance (Default|SpawnWeapon _returnvalue _weaponprop))
      (Default|AddWeapontoInventory _returnvalue _weaponprop _weaponinstance)
      (Actor|DestroyActor))))

(event EventEquipWeapon
  ;[0.122 0 0.3229 1 50] Equip Weapon
  (Collision|SetCollisionEnabled (Variables|Default|GetSphere) "NoCollision")
  (Rendering|SetActorHiddenInGame false))

(event EventBeginPlay
  (EventDispatchers|BindEventtoIsAffected? (delegate Custom|IsAffected?_Event)))

(event EventStopFire
  (bind _autofiretimer (Variables|Default|GetAutoFireTimer))
  (Utilities|IsValidTimer _autofiretimer
    (:IsValid
      (Utilities|Time|ClearandInvalidateTimerbyHandle _autofiretimer))))

(fn ConstructionScript
  (bind _weapondata (Variables|Default|GetWeaponData))
  (bind _returnvalue (Utilities|GetDataTableRow (.datatable _weapondata) (.rowname _weapondata))
    (:then
      (Variables|Default|SetWeaponProp _returnvalue)
      (Variables|Default|SetInteract%20Message (Utilities|Text|FormatText "Press \"F\" to Equip {WeaponName}" (.rowname _weapondata)))
      (Variables|Default|SetDamage (.Damage (Utilities|Struct|BreakS_WeaponMain (Variables|Default|GetWeaponProp)))))))

(fn CalculateBulletLocation
  (params (Scale :type Vector) (Target :type Scene%20Component%20Object%20Reference))
  (LocalVariables|SetForwardVerctor (Math|Vector|GetForwardVector Target))
  (LocalVariables|SetWorldLocation (Transformation|GetWorldLocation Target))
  (return (LocalVariables|GetWorldLocation) (+ (* (LocalVariables|GetForwardVerctor) (Variables|Default|GetForwardValue)) (LocalVariables|GetWorldLocation)) (Math|Transform|MakeTransform (LocalVariables|GetWorldLocation) (Math|Rotator|FindLookatRotation (LocalVariables|GetWorldLocation) (+ (* (LocalVariables|GetForwardVerctor) (Variables|Default|GetForwardValue)) (LocalVariables|GetWorldLocation))) Scale)))

(fn GetBulletLocation
  (bind _arrow (Variables|Default|GetArrow))
  (bind (_start _end) (CallFunction|BulletLocation _arrow))
  (return _start _end))

(fn DamagePlayer
  (bind _hitresult (Variables|Default|GetHitResult))
  (bind _hitactor (CallFunction|GetHitActor _hitresult))
  (Utilities|IsValid _hitactor
    (:Is%20Valid
      (bind _returnvalue (Game|Damage|ApplyDamage _hitactor (CallFunction|RecieveDamage) 0 0))
      (Development|PrintString (Utilities|String|ToString(Float) _returnvalue))
      (return))))

(fn SpawnLineTrace
  (params (Start :type Vector) (End :type Vector))
  (bind _outhit (Collision|LineTraceForObjects Start End (Variables|Default|GetObject%20Types) false (Utilities|Array|MakeArray (Variables|Default|GetOwningPlayer)) "ForDuration" true "(R=1.000000,G=0.000000,B=0.000000,A=1.000000)" "(R=0.000000,G=1.000000,B=0.000000,A=1.000000)" 1.5))
  (Variables|Default|SetHitResult _outhit)
  (return))

(fn FireFunction
  (bind (_start _end) (CallFunction|GetBulletLocation))
  (for _index (range 1 (Utilities|Struct|BreakS_WeaponMain (Variables|Default|GetWeaponProp)))
    (CallFunction|SpawnLineTrace _start _end)
    (CallFunction|DamagePlayer)
    (Class|BPICharacter|PlayAnimation(Message) (Variables|Default|GetOwningPlayer) "NewEnumerator0")))

(fn GetWeaponType
  (return (Utilities|Struct|BreakS_WeaponMain (Variables|Default|GetWeaponProp))))

(fn RecieveDamage
  (if (Variables|Default|GetIs%20Affected)
    (return (Variables|Default|GetAffected%20Damage))
    (else
      (return (Variables|Default|GetDamage)))))