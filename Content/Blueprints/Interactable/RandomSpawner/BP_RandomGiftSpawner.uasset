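; BP_RandomGiftSpawner is a one-shot spawner that replaces itself with a randomly chosen gift actor when play begins.
; On BeginPlay it spawns the gift at its own location, plays an explosion particle effect there and destroys itself.
; GetRandomGift makes a two-stage random pick: a random enum key into the Gifts map, then a random class from that entry's SpawnedActor array.
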(event EventBeginPlay
  (bind _returnvalue (Transformation|GetActorLocation))
  (|CallParentFunction)
  (Game|SpawnActorfromClass (CallFunction|GetRandomGift) (Math|Transform|MakeTransform _returnvalue "0, 0, 0" "1,1,1") "Undefined" 0 0)
  (Effects|SpawnEmitteratLocation "/Game/MobileStarterContent/Particles/P_Explosion.P_Explosion" _returnvalue)
  (Actor|DestroyActor))

(fn ConstructionScript
  (|CallParentFunction))

(fn GetRandomGift
  (return (.OutItem (Utilities|Array|Random (Utilities|Struct|BreakS_SpawnerObjects (.Value (Utilities|Map|Find (Variables|Default|GetGifts) (.OutItem (Utilities|Array|Random (Variables|Default|GetEnum))))))))))