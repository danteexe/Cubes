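; Ability variant of an interactable chest that gives a random ability pickup as its gift.
; The construction script resets the spawned actor list to hold only BP_PickupAbility.
; SpawnGiftActor draws a random data table row handle from Abilities and, if the row is found, spawns BP_PickupAbility at the chest's location with that row as its ability data.
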(event EventBeginPlay
  (|CallParentFunction) ; This node is disabled and will not be called.\nDrag off pins to build functionality.
)

(event Collision|EventActorBeginOverlap
  (params (OtherActor :type Actor%20Object%20Reference))
  (|CallParentFunction OtherActor) ; This node is disabled and will not be called.\nDrag off pins to build functionality.
)

(event EventTick
  (params (DeltaSeconds :type Float%20%28single-precision%29))
  (|CallParentFunction DeltaSeconds) ; This node is disabled and will not be called.\nDrag off pins to build functionality.
)

(fn ConstructionScript
  (|CallParentFunction)
  (Utilities|Array|Clear (Variables|Default|GetSpawnedActor))
  (Variables|Default|SetSpawnedActor (Utilities|Array|MakeArray "/Game/Blueprints/Interactable/Ability/BP_PickupAbility.BP_PickupAbility_C")))

(fn SpawnGiftActor
  (bind _abilities (Variables|Default|GetAbilities))
  (bind _outitem (Utilities|Array|Random _abilities))
  (bind _returnvalue (Utilities|GetDataTableRow (.datatable _outitem) (.rowname _outitem))
    (:then
      (Game|SpawnActorfromClass "/Game/Blueprints/Interactable/Ability/BP_PickupAbility.BP_PickupAbility_C" (Math|Transform|MakeTransform (Transformation|GetActorLocation) "0, 0, 0" "1,1,1") "Undefined" 0 _returnvalue 0)
      (return))))