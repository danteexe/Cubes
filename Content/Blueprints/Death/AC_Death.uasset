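; AC_Death is an actor component that handles the death of its owning player.
; On BeginPlay it binds to the PlayerDie dispatcher on the player's AC_HealthComponent, keeping death handling separate from health.
; The death function spawns an explosion emitter at the player's location, drops the active weapon if a valid inventory exists, then destroys the player actor.
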(event EventBeginPlay
  (|CallParentFunction)
  (EventDispatchers|AssignPlayerDie (Actor|GetComponentbyClass (Variables|Default|GetOwningPlayer) "/Game/Blueprints/Health/AC_HealthComponent.AC_HealthComponent_C") (EventDispatchers|CreateEvent :!event PlayerDeath)))

(event EventTick
  (params (DeltaSeconds :type Float%20%28single-precision%29))
  (|CallParentFunction DeltaSeconds) ; This node is disabled and will not be called.\nDrag off pins to build functionality.
)

(fn PlayerDeath
  (bind _owningplayer (Variables|Default|GetOwningPlayer))
  (bind _ac_inventory (CallFunction|GetPlayerInventory _owningplayer))
  (Effects|SpawnEmitteratLocation "/Game/MobileStarterContent/Particles/P_Explosion.P_Explosion" (Transformation|GetActorLocation (Variables|Default|GetOwningPlayer)))
  (Utilities|IsValid _ac_inventory
    (:Is%20Valid
      (Default|DropActiveWeapon _ac_inventory))
    (:Is%20Not%20Valid
      _))
  (Actor|DestroyActor (Variables|Default|GetOwningPlayer)))