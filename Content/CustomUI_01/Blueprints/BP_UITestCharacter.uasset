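; BP_UITestCharacter is a test character that brings up a custom UI sample game menu when play begins.
; BeginPlay calls CreateSampleGameMenu, which adds the Root widget to the viewport, shows the mouse cursor and sets Game and UI input mode.
; CreateDemo does the same with the WidgetsDemo widget, but its call is disconnected from any event, so it never runs.
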(event EventBeginPlay
  (CallFunction|CreateSampleGameMenu))

(fn ConstructionScript)

(fn CreateSampleGameMenu
  (bind _returnvalue (Game|GetPlayerController 0))
  (bind _returnvalue_2 (UserInterface|CreateWidget "/Game/CustomUI_01/Widgets/Root.Root_C"))
  (UserInterface|Viewport|AddtoViewport _returnvalue_2 0)
  (Variables|/Script/Engine.PlayerController|SetbShowMouseCursor _returnvalue true)
  (Input|SetInputModeGameandUI _returnvalue 0 "DoNotLock" false))

(fn CreateDemo
  (bind _returnvalue (Game|GetPlayerController 0))
  (bind _returnvalue_2 (UserInterface|CreateWidget "/Game/CustomUI_01/Widgets/WidgetsDemo.WidgetsDemo_C"))
  (UserInterface|Viewport|AddtoViewport _returnvalue_2 0)
  (Variables|/Script/Engine.PlayerController|SetbShowMouseCursor _returnvalue true)
  (Input|SetInputModeGameandUI _returnvalue 0 "DoNotLock" false))