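; Base interactable actor that tracks whether the player is within its Sphere and supplies an interaction message.
; Sphere begin and end overlap events set or clear the OnPlayer flag through an IsPlayer check that compares the actor against the player character.
; Tick also re-checks the first overlapping BP_CharacterBase, but only ever sets the flag to true.
; Getter functions expose the flag and the message.
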(event OnComponentBeginOverlap(Sphere)
  (params (OverlappedComponent :type Primitive%20Component%20Object%20Reference) (OtherActor :type Actor%20Object%20Reference) (OtherComp :type Primitive%20Component%20Object%20Reference) (OtherBodyIndex :type Integer) (bFromSweep :type Boolean) (SweepResult :type Hit%20Result%20Structure%20%28by%20ref%29))
  (Utilities|IsPlayer OtherActor
    (:True
      (Variables|Default|SetOn%20Player true))))

(event OnComponentEndOverlap(Sphere)
  (params (OverlappedComponent :type Primitive%20Component%20Object%20Reference) (OtherActor :type Actor%20Object%20Reference) (OtherComp :type Primitive%20Component%20Object%20Reference) (OtherBodyIndex :type Integer))
  (Utilities|IsPlayer OtherActor
    (:True
      (Variables|Default|SetOn%20Player false))))

(event EventBeginPlay)

(event Collision|EventActorBeginOverlap
  (params (OtherActor :type Actor%20Object%20Reference)))

(event EventTick
  (params (DeltaSeconds :type Float%20%28single-precision%29))
  (Utilities|IsPlayer (Utilities|Array|Get(acopy) (Collision|GetOverlappingActors (Variables|Default|GetSphere) "/Game/Blueprints/Character/BP_CharacterBase.BP_CharacterBase_C" :!class /Script/Engine.PrimitiveComponent))
    (:True
      (Variables|Default|SetOn%20Player true))))

(fn ConstructionScript)

(fn GetInteractMessage
  (return (Variables|Default|GetInteract%20Message)))

(fn OnPlayerCollision
  (return (Variables|Default|GetOn%20Player)))