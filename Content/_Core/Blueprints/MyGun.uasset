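; Gun actor whose mesh, body color and firing stats come from a WeaponProperties source, applied in the construction script.
; AutomaticFire runs one debug-drawn line trace per pellet from the Arrow, with random end-point spread.
; Hit Characters receive a velocity-change impulse along the horizontal impact normal, scaled by knockback power.
; A SelectBulletType macro branches hitscan versus projectile, but AutomaticFire always traces without calling it.
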(event EventBeginPlay)

(event Collision|EventActorBeginOverlap
  (params (OtherActor :type Actor%20Object%20Reference)))

(event EventTick
  (params (DeltaSeconds :type Float%20%28single-precision%29)))

(event EventAutomaticFire
  (bind _weaponproperties (Variables|Default|GetWeaponProperties))
  (bind _arrow (Variables|Default|GetArrow))
  (bind _returnvalue (Transformation|GetWorldLocation _arrow))
  (for _index (range 1 (Class|WeaponProperties|GetBulletPalletRange _weaponproperties))
    (bind _outhit (Collision|LineTraceByChannel _returnvalue (+ (+ _returnvalue (* (Math|Vector|GetForwardVector _arrow) (Class|WeaponProperties|GetDistance _weaponproperties))) (CallFunction|BulletRange 1e+02)) "TraceTypeQuery1" false 0 "ForDuration"))
    (Variables|Default|SetHitResult _outhit)
    (Variables|Default|SetImpactNormal (CallFunction|GetImpactNormal (Variables|Default|GetHitResult)))
    (CallFunction|ApplyKnocback (Variables|Default|GetHitResult))))

(fn ConstructionScript
  (bind _weaponproperties (Variables|Default|GetWeaponProperties))
  (bind _gunmesh (Variables|Default|GetGunMesh))
  (Components|SkeletalMesh|SetSkeletalMeshAsset _gunmesh (Class|WeaponProperties|GetWeaponMesh _weaponproperties))
  (Rendering|Material|SetVectorParameterValueonMaterials _gunmesh "BodyColor" (Math|Conversions|ToVector(LinearColor) (Class|WeaponProperties|GetWeaponColor _weaponproperties))))

(fn ApplyKnocback
  (params (Hit :type Hit%20Result%20Structure%20%28by%20ref%29))
  (bind _impactnormal (Variables|Default|GetImpactNormal))
  (bind (_x _y) (Math|Vector|BreakVector _impactnormal))
  (bind _ascharacter (Utilities|Casting|CastToCharacter (.HitActor (Collision|BreakHitResult Hit))))
  (Physics|AddImpulse (Variables|/Script/Engine.Character|GetCharacterMovement _ascharacter) (* (Math|Vector|MakeVector _x _y 0.0) (Class|WeaponProperties|GetKnockbackPower (Variables|Default|GetWeaponProperties))) true))

(fn BulletRange
  (params (Range :type Float%20%28double-precision%29))
  (bind _returnvalue (* Range -1.0))
  (return (Math|Vector|MakeVector (Math|Random|RandomFloatinRange _returnvalue Range) (Math|Random|RandomFloatinRange _returnvalue Range) (Math|Random|RandomFloatinRange _returnvalue Range))))