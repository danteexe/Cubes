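; BPFL_Utilities is a Blueprint function library of small shared helpers for common gameplay lookups.
; It casts to the project's game instance and player 0's character, and fetches inventory and ability components from a target actor.
; It also adds Enhanced Input mapping contexts for player 0 and unpacks hit results.
; GetImpactNormal returns the normalized trace direction from start to end, rather than the hit's surface normal.
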(fn CastGameInstance
  (params (GameInstance :type Game%20Instance%20Object%20Reference))
  (bind _asbp_game_instance (Utilities|Casting|CastToBP_GameInstance GameInstance))
  (return _asbp_game_instance))

(fn CastPlayerCharacter
  (bind _asbp_character_base (Utilities|Casting|CastToBP_CharacterBase (Game|GetPlayerCharacter 0)))
  (return _asbp_character_base))

(fn GetPlayerInventory
  (params (Target :type Character%20Object%20Reference))
  (return (Actor|GetComponentbyClass Target "/Game/Blueprints/Inventory/AC_Inventory.AC_Inventory_C")))

(fn GetPlayerAbility
  (params (Target :type Actor%20Object%20Reference))
  (return (Actor|GetComponentbyClass Target "/Game/Blueprints/Abilities/AC_Abilities.AC_Abilities_C")))

(fn AddInputMappingContext
  (params (MappingContext :type Input%20Mapping%20Context%20Object%20Reference))
  (Input|AddMappingContext (PlayerController|LocalPlayerSubsystems|GetEnhancedInputLocalPlayerSubsystem (Game|GetPlayerController 0)) MappingContext 0 "(bIgnoreAllPressedKeysUntilRelease=True,bForceImmediately=False,bNotifyUserSettings=False)"))

(fn GetImpactPoint
  (params (Hit :type Hit%20Result%20Structure%20%28by%20ref%29))
  (return (.ImpactPoint (Collision|BreakHitResult Hit))))

(fn GetHitActor
  (params (Hit :type Hit%20Result%20Structure%20%28by%20ref%29))
  (return (.HitActor (Collision|BreakHitResult Hit))))

(fn GetImpactNormal
  (params (HitResult :type Hit%20Result%20Structure%20%28by%20ref%29))
  (bind (_bblockinghit _binitialoverlap _time _distance _location _impactpoint _normal _impactnormal _physmat _hitactor _hitcomponent _hitbonename _bonename _hititem _elementindex _faceindex _tracestart _traceend) (Collision|BreakHitResult HitResult))
  (return (Math|Vector|Normalize (Math|Vector|GetUnitDirection(Vector) _tracestart _traceend))))