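; Actor component that manages a character's weapon inventory, keyed by weapon type with one active weapon.
; On BeginPlay it spawns data-table starter weapons, attaches them to the mesh's WeaponSocket and shows only the active one.
; Switching hides all weapons and messages the chosen one to equip.
; Dropping removes the entry, spawns a fresh weapon actor at a downward trace's impact point, then stops and destroys the held instance.
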(event EventBeginPlay
  (|CallParentFunction)
  (CallFunction|SpawnWeaponInventory)
  (bind _values (Utilities|Map|Values (Variables|Default|GetEquippedWeapons)))
  (for _array_element _values
    (Rendering|SetActorHiddenInGame (Utilities|Struct|BreakS_WeaponMain _array_element) true))
  (bind _returnvalue (CallFunction|GetActiveWeapon))
  (Rendering|SetActorHiddenInGame _returnvalue false))

(event EventTick
  (params (DeltaSeconds :type Float%20%28single-precision%29))
  (|CallParentFunction DeltaSeconds) ; This node is disabled and will not be called.\nDrag off pins to build functionality.
)

(event EventEndPlay
  (params (EndPlayReason :type EEndPlayReason%20Enum :default "Destroyed")))

(event EventDropWeapon
  (params (DroppedWeaponData :type S%20Weapon%20Main%20Structure))
  (CallFunction|DropEquippedWepaon DroppedWeaponData))

(event EventDropActiveWeapon
  (CallFunction|DropEquippedWepaon (.Value (Utilities|Map|Find (Variables|Default|GetEquippedWeapons) (Variables|Default|GetActiveWeapon)))))

(fn SpawnWeaponInventory
  (bind _values (Utilities|Map|Values (Variables|Default|GetStartedWeapon)))
  (for _array_element _values
    (bind _returnvalue (Utilities|GetDataTableRow (.datatable _array_element) (.rowname _array_element))
      (:then
        (bind _findedweapon (Utilities|FindEquippedWeapon _returnvalue)
          (:Finded
            (CallFunction|DropEquippedWepaon _findedweapon))
          (:NotFinded
            _))
        (bind _weaponinstance (CallFunction|SpawnWeapon _returnvalue))
        (CallFunction|AddWeapontoInventory _returnvalue _weaponinstance)))))

(fn SpawnWeapon
  (params (SpawnedWeapon :type S%20Weapon%20Main%20Structure))
  (bind _returnvalue (Game|SpawnActorfromClass (Utilities|Struct|BreakS_WeaponMain SpawnedWeapon) (Math|Transform|MakeTransform "0, 0, 0" "0, 0, 0" "1,1,1") "Undefined" 0 (Variables|Default|GetOwningPlayer) 0))
  (Collision|SetCollisionEnabled (Variables|/Game/_Core/Blueprints/Interactable/BP_InteractableBase.BP_InteractableBase_C|GetSphere _returnvalue) "NoCollision")
  (Transformation|AttachComponentToComponent _returnvalue (Variables|/Script/Engine.Character|GetMesh (Variables|Default|GetOwningPlayer)) "WeaponSocket" "SnapToTarget" "SnapToTarget" "KeepWorld" true)
  (Rendering|SetActorHiddenInGame _returnvalue false)
  (return _returnvalue))

(fn AddWeapontoInventory
  (params (AddedWeapon :type S%20Weapon%20Main%20Structure) (WeaponInstance :type BP%20Weapon%20Base%20Object%20Reference))
  (bind _weapontype (Utilities|Struct|BreakS_WeaponMain AddedWeapon))
  (bind _structout (Utilities|Struct|SetmembersinS_WeaponMain AddedWeapon WeaponInstance))
  (Utilities|Map|Add (Variables|Default|GetEquippedWeapons) _weapontype _structout)
  (Variables|Default|SetActiveWeapon _weapontype))

(fn DropEquippedWepaon
  (params (DroppedWeapon :type S%20Weapon%20Main%20Structure%20%28by%20ref%29))
  (bind _owningplayer (Variables|Default|GetOwningPlayer))
  (bind _returnvalue (Transformation|GetActorLocation _owningplayer))
  (bind (_x _y _z) (Math|Vector|BreakVector _returnvalue))
  (bind _findedweapon (Utilities|FindEquippedWeapon DroppedWeapon)
    (:Finded
      (LocalVariables|Settmp_Data _findedweapon)
      (Utilities|IsValid (Utilities|Struct|BreakS_WeaponMain (LocalVariables|Gettmp_Data))
        (:Is%20Valid
          (LocalVariables|Settmp_Weapon (Utilities|Struct|BreakS_WeaponMain (LocalVariables|Gettmp_Data)))
          (CallFunction|RemoveWeaponfromInventory (LocalVariables|Gettmp_Data))
          (bind _outhit (Collision|LineTraceByChannel _returnvalue (Math|Vector|MakeVector _x _y (- _z 2e+02)) "TraceTypeQuery1" false 0 "None" true "(R=1.000000,G=0.000000,B=0.000000,A=1.000000)" "(R=0.000000,G=1.000000,B=0.000000,A=1.000000)" 1e+01))
          (Game|SpawnActorfromClass (Utilities|Struct|BreakS_WeaponMain (LocalVariables|Gettmp_Data)) (Math|Transform|MakeTransform (CallFunction|GetImpactPoint _outhit) "0, 0, 0" "1,1,1") "Undefined" 0 (Variables|Default|GetOwningPlayer) 0)
          (bind _tmp_weapon (LocalVariables|Gettmp_Weapon)
            (:then
              (Class|BPIWeapon|StopFire(Message) _tmp_weapon)
              (Actor|DestroyActor _tmp_weapon))
            (:else)))))))

(fn RemoveWeaponfromInventory
  (params (RemovedWeapon :type S%20Weapon%20Main%20Structure%20%28by%20ref%29))
  (Utilities|Map|Remove (Variables|Default|GetEquippedWeapons) (Utilities|Struct|BreakS_WeaponMain RemovedWeapon)))

(fn ChangeWeapon
  (params (EquippedWeapon :type E_WeaponType%20Enum :default "NewEnumerator0"))
  (bind _equippedweapons (Variables|Default|GetEquippedWeapons))
  (bind (_value _returnvalue) (Utilities|Map|Find _equippedweapons EquippedWeapon))
  (bind _weaponinstance (Utilities|Struct|BreakS_WeaponMain _value))
  (if _returnvalue
    (bind _values (Utilities|Map|Values _equippedweapons))
    (for _array_element _values
      (Utilities|IsValid (Utilities|Struct|BreakS_WeaponMain _array_element)
        (:Is%20Valid
          (Rendering|SetActorHiddenInGame (Utilities|Struct|BreakS_WeaponMain _array_element) true))))
    (Variables|Default|SetActiveWeapon EquippedWeapon)
    (Utilities|IsValid _weaponinstance
      (:Is%20Valid
        (Class|BPIWeapon|EquipWeapon(Message) _weaponinstance)))))

(fn GetActiveWeapon
  (return (Utilities|Struct|BreakS_WeaponMain (.Value (Utilities|Map|Find (Variables|Default|GetEquippedWeapons) (Variables|Default|GetActiveWeapon))))))