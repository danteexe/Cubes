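; Inventory component that gives its owning Character a set of starting weapons when play begins.
; Each StartedWeapon entry supplies an actor class and a hand socket name, and the spawned actor attaches to the Character's mesh at that socket.
; An empty list prints an on-screen warning.
; Spawned weapons are not stored, and no other inventory logic is present.
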(event EventBeginPlay
  (bind _startedweapon (Variables|Default|GetStartedWeapon))
  (if (Utilities|Array|IsNotEmpty _startedweapon)
    (for _array_element _startedweapon
      (bind _returnvalue (Game|SpawnActorfromClass (Class|WeaponProperties|GetWeaponInstance _array_element) (Math|Transform|MakeTransform "0, 0, 0" "0, 0, 0" "1.000000,1.000000,1.000000") "Undefined" "MultiplyWithRoot" 0 0))
      (Transformation|AttachComponentToComponent _returnvalue (Variables|/Script/Engine.Character|GetMesh (.AsCharacter (Utilities|Casting|CastToCharacter (Components|GetOwner)))) (Class|WeaponProperties|GetHandSocketName _array_element) "KeepRelative" "KeepRelative" "KeepRelative" true))
    (else
      (Development|PrintString "Started Weapon is Empty - AC_Inventory" true true "(R=1.000000,G=0.000000,B=0.012904,A=1.000000)" 5.0))))

(event EventTick
  (params (DeltaSeconds :type Float%20%28single-precision%29)))