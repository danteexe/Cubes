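; BP_ActorBase is a base player character with world-axis movement, a health component and a health bar widget.
; BeginPlay hands itself to the health bar widget and adds an input mapping context, while movement uses legacy axis events.
; RecieveHealth forwards health changes to HealthComp, and getters expose the character and its current health.
; The construction script tints the mesh through a dynamic material instance using the Color variable.
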(event EventBeginPlay
  (Class|BPIHealthBar|SetOwningCharacter(Message) (UserInterface|GetUserWidgetObject (Variables|Default|GetHealthBar)) self)
  (CallFunction|AddInputMappingContext (Variables|Default|GetMapping%20Context)))

(event Collision|EventActorBeginOverlap
  (params (OtherActor :type Actor%20Object%20Reference)))

(event EventTick
  (params (DeltaSeconds :type Float%20%28single-precision%29)))

(event EventRecieveHealth
  (params (Recieve%20Type :type E_HealthRecieveType%20Enum :default "NewEnumerator0") (Values :type Float%20%28single-precision%29))
  (Default|RecieveHealth (Variables|Default|GetHealthComp) Recieve%20Type Values))

(event Input|AxisEvents|InputAxisMoveForward
  (params (AxisValue :type Float%20%28single-precision%29))
  ;[0.1968 1 0.9602 1 50] Movement
  (Pawn|Input|AddMovementInput "1.000000, 0, 0" AxisValue false))

(event Input|AxisEvents|InputAxisMoveRight
  (params (AxisValue :type Float%20%28single-precision%29))
  ;[0.1968 1 0.9602 1 50] Movement
  (Pawn|Input|AddMovementInput "0,1.000000, 0" AxisValue false))

(fn ConstructionScript
  (bind _returnvalue (Rendering|Material|CreateDynamicMaterialInstance (Variables|Character|GetMesh) 0 "/Game/Materials/M_BaseColor.M_BaseColor" "" :!class /Script/Engine.PrimitiveComponent))
  (Rendering|Material|SetVectorParameterValue _returnvalue "BaseColor" (Variables|Default|GetColor) :!class /Script/Engine.MaterialInstanceDynamic))

(fn GetPlayerCharacter
  (return self))

(fn GetPlayerCurrentHealth
  (return (Variables|/Game/Blueprints/Health/AC_HealthComponent.AC_HealthComponent_C|GetCurrentHealth (Variables|Default|GetHealthComp))))